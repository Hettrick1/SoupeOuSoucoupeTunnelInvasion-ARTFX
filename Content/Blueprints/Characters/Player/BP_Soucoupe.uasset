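; BP_Soucoupe is a player flying saucer that rotates in steps, detects hits and adds score.
; Rotate wraps a target index across eight 45-degree steps, and a timeline scaled by game speed lerps the root's pitch along the shortest path.
; Overlaps tagged Laser or Boost send hit or boost messages to the player pawn.
; SetScore adds the boost multiplier to the game instance score, fetched through the pawn.
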(event `Rotate`
  (params (gameSpeed :type "Float (double-precision)") (rotation :type Integer))
  (bind _defaultsceneroot (`self.DefaultSceneRoot`))
  ;[1 1 1] Rotate
  (`TimelineComponent.SetPlayRate` (`self.lerpRotation`) (* gameSpeed 3.0))
  (bind _output_get (set `self.targetRotation` (+ (`self.targetRotation`) rotation)))
  (if (< _output_get 0)
    (set `self.targetRotation` 7)
    (bind (_direction _lerp) (`Timeline|lerpRotation` :!via `PlayFromStart` :!label _label)
      (:`Update`
        (`SceneComponent.K2_SetRelativeRotation` _defaultsceneroot (`KismetMathLibrary.RLerp` (`SceneComponent.RelativeRotation` _defaultsceneroot) (`KismetMathLibrary.MakeRotator` 0.0 (* (`self.targetRotation`) 45.0)) _lerp true) false false)))
    (elif (> _output_get 7)
      (set `self.targetRotation` 0)
      (goto _label :!via `PlayFromStart`)
      (else
        (goto _label :!via `PlayFromStart`)))))

(event `self.Collision.OnComponentBeginOverlap`
  (params (OverlappedComponent :type "PrimitiveComponent Object Reference") (OtherActor :type "Actor Object Reference") (OtherComp :type "PrimitiveComponent Object Reference") (OtherBodyIndex :type Integer) (bFromSweep :type Boolean) (SweepResult :type "HitResult Structure (by ref)"))
  (bind _returnvalue (`GameplayStatics.GetPlayerPawn` 0))
  ;[1 1 1] GetHit
  (`/Engine/EditorBlueprintResources/StandardMacros.IsValid` OtherActor
    (:`Is Valid`
      (if (`self.ActorHasTag` OtherActor "Laser")
        (message `/Game/Blueprints/Characters/BPI/BPI_Player.PlayerHit` _returnvalue)
        (elif (`self.ActorHasTag` OtherActor "Boost")
          (message `/Game/Blueprints/Characters/BPI/BPI_Player.GetBoost` _returnvalue))))))

(event `/Game/Blueprints/Characters/BPI/BPI_Player.SetScore`
  ;[1 1 1] Set score
  (bind _giref (message `/Game/Blueprints/Characters/BPI/BPI_Player.GetGameInstance` (`GameplayStatics.GetPlayerPawn` 0)))
  (set `/Game/_Manager/InGame/GI_SOS.score` (+ (`/Game/_Manager/InGame/GI_SOS.score` _giref) (`/Game/_Manager/InGame/GI_SOS.boostScoreMultiplier` _giref)) _giref))

(fn `GetGameInstance`
  (returns (giRef :type "/Game/_Manager/InGame/GI_SOS Object Reference"))
  (return null))

(fn `GetGameSpeed`
  (returns (gameSpeed :type "Float (double-precision)"))
  (return 0.0))

(fn `UserConstructionScript`)