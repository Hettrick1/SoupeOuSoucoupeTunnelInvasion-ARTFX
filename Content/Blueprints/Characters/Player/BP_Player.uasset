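; BP_Player is the player Blueprint, which spawns and steers a BP_Soucoupe (saucer) and tracks lives.
; On BeginPlay it spawns the saucer at its own transform and keeps a reference to it.
; Move forwards direction and game speed to the saucer's Rotate.
; PlayerHit decrements Lives with nothing yet happening at zero, and the MPC_WorldParameter setter nodes are unconnected.
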(event `self.ReceiveBeginPlay`
  ;[1 1 1] Create soucoupe
  (bind _returnvalue (`|SpawnActorFromClass` "/Game/Blueprints/Characters/Player/BP_Soucoupe.BP_Soucoupe_C" (`self.GetTransform`) "AlwaysSpawn" "MultiplyWithRoot" null null))
  (set `self.soucoupeRef` _returnvalue))

(event `/Game/Blueprints/Characters/BPI/BPI_Player.Move`
  (params (direction :type Integer))
  (bind _soucouperef (`self.soucoupeRef`))
  ;[1 1 1] Rotate
  (`/Engine/EditorBlueprintResources/StandardMacros.IsValid` _soucouperef
    (:`Is Valid`
      (`/Game/Blueprints/Characters/Player/BP_Soucoupe.Rotate` _soucouperef (`self.gameSpeed`) direction))))

(event `/Game/Blueprints/Characters/BPI/BPI_Player.PlayerHit`
  ;[1 1 1] Damage
  (bind _result (`/Engine/EditorBlueprintResources/StandardMacros.DecrementInt` (`self.lives`))
    (:`  `
      (if (<= _result 0)
        _))))

(fn `UserConstructionScript`
  (`parent.UserConstructionScript`))