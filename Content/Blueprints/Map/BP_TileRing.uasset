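; BP_TileRing is a map actor that configures a ring of eight child-actor tiles from a ring template.
; Shortly after BeginPlay, SetRingType maps the template value to one of five predefined tile-type arrays.
; SetTileType then sends each tile its entry by index through SetTileMessage.
; GetTemplate exposes the ring's current Template value.
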(event `self.ReceiveBeginPlay`
  (`KismetSystemLibrary.Delay` 0.2)
  (`/Game/Blueprints/BPI/BPI_Tile.SetRingType` (`self.template`)))

(event `/Game/Blueprints/BPI/BPI_Tile.SetRingType`
  (params (NewParam :type "/Game/Blueprints/Enums/Enum_RingType Enum" :default "NewEnumerator0"))
  (`self.SetTileType` (select `/Game/Blueprints/Enums/Enum_RingType` NewParam :`NewEnumerator0` (`self.template0`) :`NewEnumerator1` (`self.template1`) :`NewEnumerator2` (`self.template2`) :`NewEnumerator3` (`self.template3`) :`NewEnumerator4` (`self.template4`))))

(fn `GetTemplate`
  (returns (template :type "/Game/Blueprints/Enums/Enum_RingType Enum"))
  (return (`self.template`)))

(fn `SetTileType`
  (params (childType :type "Array of Actor Class Reference"))
  (for (_array_element _array_index) (`|MakeArray` (`ChildActorComponent.ChildActor` (`self.Tile1`)) (`ChildActorComponent.ChildActor` (`self.Tile2`)) (`ChildActorComponent.ChildActor` (`self.Tile3`)) (`ChildActorComponent.ChildActor` (`self.Tile4`)) (`ChildActorComponent.ChildActor` (`self.Tile5`)) (`ChildActorComponent.ChildActor` (`self.Tile6`)) (`ChildActorComponent.ChildActor` (`self.Tile7`)) (`ChildActorComponent.ChildActor` (`self.Tile8`)))
    (message `/Game/Blueprints/BPI/BPI_Tile.SetTile` _array_element (`|GetArrayItem` (`local.childType`) _array_index))))

(fn `UserConstructionScript`)