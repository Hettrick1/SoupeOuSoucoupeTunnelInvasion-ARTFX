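; BP_TunelManager builds an endlessly scrolling tunnel from recycled BP_TileRing actors.
; On BeginPlay it spawns evenly spaced rings along Y, starting four behind itself, all sharing one dynamic material, and caches both end locations.
; Each Tick moves rings a fixed, frame-rate-dependent step against their right vector.
; Rings passing the first cached location snap to the last, forming a treadmill loop without respawning.
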(event `self.ReceiveBeginPlay`
  (bind _allrings (`self.allRings`))
  (bind _returnvalue (`KismetMaterialLibrary.CreateDynamicMaterialInstance` "/DatasmithContent/Materials/AliasReference.AliasReference"))
  (set `self.dynamicMaterial` _returnvalue)
  (for _index (range -4 (+ (`self.nbreOfRings`) 1))
    (bind _returnvalue_2 (`|SpawnActorFromClass` "/Game/Blueprints/Map/BP_TileRing.BP_TileRing_C" (`KismetMathLibrary.Conv_VectorToTransform` (+ (`self.K2_GetActorLocation`) (`KismetMathLibrary.MakeVector` 0.0 (* _index (`self.spaceBetweenRings`))))) "AlwaysSpawn" "MultiplyWithRoot" null (`self.dynamicMaterial`) null))
    (`KismetArrayLibrary.Array_Add` (`self.allRings`) _returnvalue_2))
  (set `self.firstRingLocation` (`self.K2_GetActorLocation` (`|GetArrayItem` _allrings)))
  (set `self.lastRingLocation` (`self.K2_GetActorLocation` (`|GetArrayItem` _allrings (- (`KismetArrayLibrary.Array_Length` _allrings) 1)))))

(event `self.ReceiveTick`
  (params (DeltaSeconds :type "Float (single-precision)"))
  (bind (_firstringlocation_x _firstringlocation_y) (`KismetMathLibrary.BreakVector` (`self.firstRingLocation`)))
  (for _array_element (`self.allRings`)
    (`self.K2_SetActorLocation` _array_element (+ (`self.K2_GetActorLocation` _array_element) (* (`self.GetActorRightVector` _array_element) -10.0)) false false)
    (bind (_returnvalue_x _returnvalue_y) (`KismetMathLibrary.BreakVector` (`self.K2_GetActorLocation` _array_element)))
    (if (< _returnvalue_y _firstringlocation_y)
      (`self.K2_SetActorLocation` _array_element (`self.lastRingLocation`) false false))))

(fn `UserConstructionScript`)