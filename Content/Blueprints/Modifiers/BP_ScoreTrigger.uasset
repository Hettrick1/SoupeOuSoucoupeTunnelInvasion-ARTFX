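; BP_ScoreTrigger is a box trigger that registers a score when a player actor overlaps it.
; The first overlap by an actor implementing BPI_Player passes a DoOnce, so each trigger fires a single time.
; It then plays the HUD_Game widget's Bounce animation and sends SetScoreMessage to that actor, both dependent on the HUD cast succeeding.
; Score force feedback follows if the game instance, fetched through the player pawn, has rumble enabled.
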(event `self.Box.OnComponentBeginOverlap`
  (params (OverlappedComponent :type "PrimitiveComponent Object Reference") (OtherActor :type "Actor Object Reference") (OtherComp :type "PrimitiveComponent Object Reference") (OtherBodyIndex :type Integer) (bFromSweep :type Boolean) (SweepResult :type "HitResult Structure (by ref)"))
  (if (`KismetSystemLibrary.DoesImplementInterface` OtherActor "/Game/Blueprints/Characters/BPI/BPI_Player.BPI_Player_C")
    (`/Engine/EditorBlueprintResources/StandardMacros.DoOnce` false
      (:`Completed`
        (bind _ashud_game (cast `/Game/_Manager/InGame/HUD_Game` (`PlayerController.GetHUD` (`GameplayStatics.GetPlayerController` 0))))
        (bind _widgetref (`/Game/_Manager/InGame/HUD_Game.widgetRef` _ashud_game))
        (`UserWidget.PlayAnimation` _widgetref (`/Game/UI/Widgets/WBP_PlayerHUD.Bounce` _widgetref) 0.0 1 "Forward" 1.0 true)
        (message `/Game/Blueprints/Characters/BPI/BPI_Player.SetScore` OtherActor)
        (bind _giref (message `/Game/Blueprints/Characters/BPI/BPI_Player.GetGameInstance` (`GameplayStatics.GetPlayerPawn` 0)))
        (if (`/Game/_Manager/InGame/GI_SOS.hasRumble` _giref)
          (`PlayerController.K2_ClientPlayForceFeedback` (`GameplayStatics.GetPlayerController` 0) "/Game/Haptic/FFE_Score.FFE_Score" "None" false false false))))))

(fn `UserConstructionScript`
  (`parent.UserConstructionScript`))